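; Static helper library for the in-game smartphone and device system, covering app launching, widget focus, device lookup and messaging.
; Recursive widget-tree searches locate buttons and panels for focus navigation, alongside helpers for on-screen device roots, active camera and key icons.
; SendTextMessage files texts into dialogues on the pawn's BP_SmartphoneComponent, refreshes an open Messages app and calls SendNotification.
; SendNotification logs and shows a popup positioned by viewport scaling from 1920x1080.
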(fn `FindAllButtonsUnderThePanel`
  (params (Root :type "Widget Object Reference"))
  (returns (Buttons :type "Array of Widget Object Reference"))
  (locals (RootAsPanel :type "PanelWidget Object Reference") (Out :type "Array of Widget Object Reference") (LastChild :type "Widget Object Reference"))
  (`|ExecutionSequence`
    (:`then_0`
      (bind _aspanel_widget (cast `PanelWidget` Root)
        (:`then`
          (bind _output_get (set `local.RootAsPanel` _aspanel_widget))
          (for _index (range (`PanelWidget.GetChildrenCount` _output_get))
            (bind _output_get_2 (set `local.LastChild` (`PanelWidget.GetChildAt` (`local.RootAsPanel`) _index)))
            (bind _asbutton (cast `Button` _output_get_2)
              (:`then`
                (`KismetArrayLibrary.Array_Add` (`local.Out`) _asbutton))
              (:`CastFailed`
                (bind _buttons (`self.FindAllButtonsUnderThePanel` (`local.LastChild`) (`local.__WorldContext`)))
                (`KismetArrayLibrary.Array_Append` (`local.Out`) _buttons)))))
        (:`CastFailed`
          (bind _asuser_widget (cast `UserWidget` Root))
          (if (`UserWidget.bIsFocusable` _asuser_widget)
            (return (`|MakeArray` _asuser_widget :!type "Widget Object Reference"))))))
    (:`then_1`
      (return (`local.Out`)))))

(fn `FindDeviceComponent`
  (params (PawnReference :type "Actor Object Reference") (DeviceClass :type "/Game/Smartphone/BP/BP_DeviceActor Class Reference"))
  (returns (DevComp :type "/Game/Smartphone/BP/DeviceComponents/BP_DeviceComponent Object Reference"))
  (for _array_element (`Actor.K2_GetComponentsByClass` PawnReference "/Game/Smartphone/BP/DeviceComponents/BP_DeviceComponent.BP_DeviceComponent_C")
    (`/Game/Smartphone/BP/DeviceComponents/BP_DeviceComponent.AnimationBP_Ref` _array_element
      (:`then`)
      (:`else`
        (if (== (`/Game/Smartphone/BP/DeviceComponents/BP_DeviceComponent.DeviceClass` _array_element) DeviceClass)
          (return _array_element)))))
  (return null))

(fn `FindPanelWithRequiredButton`
  (params (Root :type "Widget Object Reference") (ButtonClass :type "UserWidget Class Reference") (`include default Button class` :type Boolean) (ShouldHaveChildWithFocus :type Boolean))
  (returns (OutputPin :type "Widget Object Reference"))
  (locals (LastChild :type "Widget Object Reference") (LastPanel :type "PanelWidget Object Reference"))
  (bind _aspanel_widget (cast `PanelWidget` Root))
  (for _array_element (`PanelWidget.GetAllChildren` _aspanel_widget)
    (if ShouldHaveChildWithFocus
      (if (or (`Widget.HasAnyUserFocus` _array_element) (`Widget.HasFocusedDescendants` _array_element))
        (bind _asuser_widget (cast `UserWidget` _array_element :!label _label)
          (:`then`
            (if (== (`GameplayStatics.GetObjectClass` _asuser_widget) ButtonClass)
              (return Root)
              (else
                _)))
          (:`CastFailed`
            _))
        (if `include default Button class`
          (bind _asbutton (cast `Button` _array_element)
            (:`then`
              (return _asbutton))
            (:`CastFailed`
              _)))
        (bind _outputpin (`self.FindPanelWithRequiredButton` _array_element ButtonClass `include default Button class` ShouldHaveChildWithFocus (`local.__WorldContext`)))
        (return _outputpin))
      (else
        (goto _label)))))

(fn `FindPanelWithRequiredButtons`
  (params (Root :type "Widget Object Reference") (ButtonClass :type "Array of UserWidget Class Reference") (`include default Button class` :type Boolean) (ShouldHaveChildWithFocus :type Boolean))
  (returns (OutputPin :type "Widget Object Reference"))
  (locals (LastChild :type "Widget Object Reference") (LastPanel :type "PanelWidget Object Reference") (LastFound :type "Widget Object Reference"))
  (for _array_element ButtonClass
    (bind _outputpin (`self.FindPanelWithRequiredButton` Root _array_element `include default Button class` ShouldHaveChildWithFocus (`local.__WorldContext`)))
    (bind _output_get (set `local.LastFound` _outputpin))
    (`/Engine/EditorBlueprintResources/StandardMacros.IsValid` _output_get
      (:`Is Valid`
        (return _output_get)))))

(fn `FocusOnButton`
  (params (NewFocused :type "Widget Object Reference"))
  (bind _root (`self.GetRootWidgets` null (`local.__WorldContext`)))
  (message `/Game/Smartphone/BP/BP_DevicesInterface.UpdateLastFocusedWidget` (`/Game/Smartphone/UMG/UMG_OnScreenDevice.DeviceWidget` _root) NewFocused false))

(fn `Get Name From App Class`
  (params (InClass :type "UserWidget Class Reference"))
  (returns (Output_Get :type String))
  (locals (InName :type String))
  (bind _inname (`local.InName`))
  (set `local.InName` (`KismetSystemLibrary.GetClassDisplayName` InClass))
  (if (`KismetStringLibrary.StartsWith` (`local.InName`) "UMG_SP_" "CaseSensitive")
    (bind _output_get (set `local.InName` (`KismetStringLibrary.Right` _inname (- (`KismetStringLibrary.Len` _inname) 7))))
    (if (`KismetStringLibrary.EndsWith` _output_get "_C" "CaseSensitive")
      (bind _output_get_2 (set `local.InName` (`KismetStringLibrary.Left` _output_get (- (`KismetStringLibrary.Len` _output_get) 2))))
      (return _output_get_2))))

(fn `GetActiveCamera`
  (params (Target :type "Actor Object Reference"))
  (returns (ActiveCamera :type "CameraComponent Object Reference"))
  (for _array_element (`Actor.K2_GetComponentsByClass` Target "/Script/Engine.CameraComponent")
    (if (`ActorComponent.IsActive` _array_element)
      (return _array_element))))

(fn `GetKeysImages`
  (returns (OutMapping :type "Map of Key Structure to Texture2D Object Reference"))
  (return (`|MakeMap` "LeftMouseButton" "/Game/Smartphone/Texture/ControllerIcons/T_UI_LMB.T_UI_LMB" "RightMouseButton" "/Game/Smartphone/Texture/ControllerIcons/T_UI_RMB.T_UI_RMB" "Gamepad_FaceButton_Bottom" "/Game/Smartphone/Texture/ControllerIcons/T_UI_gp_A.T_UI_gp_A" "Gamepad_FaceButton_Right" "/Game/Smartphone/Texture/ControllerIcons/T_UI_gp_B.T_UI_gp_B" "Gamepad_FaceButton_Left" "/Game/Smartphone/Texture/ControllerIcons/T_UI_gp_X.T_UI_gp_X" "Gamepad_FaceButton_Top" "/Game/Smartphone/Texture/ControllerIcons/T_UI_gp_Y.T_UI_gp_Y" "Gamepad_RightShoulder" "/Game/Smartphone/Texture/ControllerIcons/T_UI_gp_RB.T_UI_gp_RB" "Gamepad_LeftShoulder" "/Game/Smartphone/Texture/ControllerIcons/T_UI_gp_LB.T_UI_gp_LB" "Gamepad_RightTrigger" "/Game/Smartphone/Texture/ControllerIcons/T_UI_gp_RT.T_UI_gp_RT" "Gamepad_LeftTrigger" "/Game/Smartphone/Texture/ControllerIcons/T_UI_gp_LT.T_UI_gp_LT" "Gamepad_DPad_Up" "/Game/Smartphone/Texture/ControllerIcons/T_UI_gp_DPAD_U.T_UI_gp_DPAD_U" "Gamepad_DPad_Down" "/Game/Smartphone/Texture/ControllerIcons/T_UI_gp_DPAD_D.T_UI_gp_DPAD_D" "Gamepad_DPad_Right" "/Game/Smartphone/Texture/ControllerIcons/T_UI_gp_DPAD_R.T_UI_gp_DPAD_R" "Gamepad_DPad_Left" "/Game/Smartphone/Texture/ControllerIcons/T_UI_gp_DPAD_L.T_UI_gp_DPAD_L" :!type "Key Structure" :!valuetype "Texture2D Object Reference")))

(fn `GetRootWidgets`
  (params (DeviceHomeWidgetClass :type "Object Class Reference"))
  (returns (Root :type "/Game/Smartphone/UMG/UMG_OnScreenDevice Object Reference") (DeviceWidget :type "UserWidget Object Reference"))
  (locals (AllFoundWidgets :type "Array of /Game/Smartphone/UMG/UMG_OnScreenDevice Object Reference"))
  (bind _output (`|GetArrayItem` (`local.AllFoundWidgets`)))
  (if (`KismetSystemLibrary.IsValidClass` DeviceHomeWidgetClass)
    (bind _foundwidgets (`WidgetBlueprintLibrary.GetAllWidgetsOfClass` (`local.__WorldContext`) "/Game/Smartphone/UMG/UMG_OnScreenDevice.UMG_OnScreenDevice_C"))
    (for _array_element _foundwidgets
      (bind _devicewidget (`/Game/Smartphone/UMG/UMG_OnScreenDevice.DeviceWidget` _array_element))
      (if (== (`GameplayStatics.GetObjectClass` _devicewidget) DeviceHomeWidgetClass)
        (return _array_element _devicewidget)))
    (else
      (bind _foundwidgets_2 (`WidgetBlueprintLibrary.GetAllWidgetsOfClass` (`local.__WorldContext`) "/Game/Smartphone/UMG/UMG_OnScreenDevice.UMG_OnScreenDevice_C"))
      (bind _output_get (set `local.AllFoundWidgets` _foundwidgets_2))
      (if (== (`KismetArrayLibrary.Array_Length` _output_get) 0)
        (return null null)
        (else
          (return _output (`/Game/Smartphone/UMG/UMG_OnScreenDevice.DeviceWidget` _output)))))))

(fn `OpenSmartphoneApp`
  (params (App :type "UserWidget Class Reference") (Container :type "PanelWidget Object Reference"))
  (returns (CreatedWidget1 :type "UserWidget Object Reference"))
  (locals (CreatedWidget :type "UserWidget Object Reference"))
  (bind _createdwidget (`local.CreatedWidget`))
  (if (`KismetSystemLibrary.IsValidClass` App)
    (bind _returnvalue (`|CreateWidget` App))
    (bind _output_get (set `local.CreatedWidget` _returnvalue))
    (`PanelWidget.AddChild` Container _output_get)
    (set `UserWidget.bIsFocusable` true _createdwidget)
    (`Widget.SetUserFocus` (`local.CreatedWidget`) (`Widget.GetOwningPlayer` Container))
    (return _createdwidget)))

(fn `ScaleUMG Position`
  (params (InVec :type "Vector2D Structure (by ref)"))
  (returns (ReturnValue :type "Vector2D Structure"))
  (bind (_x _y) (`KismetMathLibrary.BreakVector2D` InVec))
  (bind _returnvalue_x (`KismetMathLibrary.BreakVector2D` (`WidgetLayoutLibrary.GetViewportSize` (`local.__WorldContext`))))
  (bind (_returnvalue_x_2 _returnvalue_y) (`KismetMathLibrary.BreakVector2D` (`WidgetLayoutLibrary.GetViewportSize` (`local.__WorldContext`))))
  (return (`KismetMathLibrary.MakeVector2D` (`KismetMathLibrary.MapRangeUnclamped` _returnvalue_x 0.0 1920.0 0.0 _x) (`KismetMathLibrary.MapRangeUnclamped` _returnvalue_y 0.0 1080.0 0.0 _y))))

(fn `SearchForRequiredButton`
  (params (startIndex :type Integer) (EndIndex :type Integer) (ReverseLoop :type Boolean) (AllowedClasses :type "Array of UserWidget Class Reference") (ReferenceArray :type "Array of Widget Object Reference"))
  (returns (Output :type Integer) (OutWidget :type "Widget Object Reference"))
  (locals (CurrI :type Integer :default 0))
  (for _index (range startIndex (+ EndIndex 1))
    (set `local.CurrI` (`KismetMathLibrary.SelectInt` (- EndIndex _index) _index ReverseLoop))
    (bind _asuser_widget (cast `UserWidget` (`|GetArrayItem` (`local.ReferenceArray`) (`local.CurrI`))))
    (if (`KismetArrayLibrary.Array_Contains` AllowedClasses (`GameplayStatics.GetObjectClass` _asuser_widget))
      (return (`local.CurrI`) (`|GetArrayItem` (`local.ReferenceArray`) (`local.CurrI`)))))
  (return -1 null))

(fn `SendNotification`
  (params (To :type "PlayerController Object Reference") (Title :type Text) (NotifText :type Text) (App :type "/Game/Smartphone/Structures/SmartphoneApp_Struct Structure"))
  (returns (Notification :type "/Game/Smartphone/UMG/DevicesBases/SmartphoneFeatures/NotifCenter/UMG_Notification Object Reference"))
  (locals (`Screen SIze` :type "Vector2D Structure") (SmartphoneCompRef :type "/Game/Smartphone/BP/DeviceComponents/BP_SmartphoneComponent Object Reference") (CreatedNotification :type "/Game/Smartphone/UMG/DevicesBases/SmartphoneFeatures/NotifCenter/UMG_Notification Object Reference") (ScreenPosition :type "Vector2D Structure"))
  (bind _screen_size_x (`KismetMathLibrary.BreakVector2D` (`local.Screen SIze`)))
  (bind (_ui_class _screenmaterialname _screenmaterialparameter _ui_screensize _ui_screenposition) (defaults `Object` (`/Game/Smartphone/BP/DeviceComponents/BP_DeviceComponent.DeviceClass` (`local.SmartphoneCompRef`))))
  (`/Engine/EditorBlueprintResources/StandardMacros.IsValid` To
    (:`Is Valid`
      (bind _output_get (set `local.SmartphoneCompRef` (`Actor.GetComponentByClass` (`Controller.K2_GetPawn` To) "/Game/Smartphone/BP/DeviceComponents/BP_SmartphoneComponent.BP_SmartphoneComponent_C")))
      (`/Engine/EditorBlueprintResources/StandardMacros.IsValid` _output_get
        (:`Is Valid`
          (set `local.Screen SIze` _ui_screensize)
          (set `local.ScreenPosition` _ui_screenposition)
          (bind _returnvalue (`|CreateWidget` "/Game/Smartphone/UMG/DevicesBases/SmartphoneFeatures/NotifCenter/UMG_Notification.UMG_Notification_C" (`local.To`) 5.0 (`local.App`) (`local.Title`) (`local.NotifText`)))
          (set `local.CreatedNotification` _returnvalue)
          (bind _creatednotification (`local.CreatedNotification`)
            (:`then`
              (`UserWidget.AddToPlayerScreen` _creatednotification 1)
              (`UserWidget.SetDesiredSizeInViewport` (`local.CreatedNotification`) (`KismetMathLibrary.MakeVector2D` (/ _screen_size_x 2.0) 100.0))
              (`UserWidget.SetPositionInViewport` (`local.CreatedNotification`) (`self.ScaleUMG Position` (`local.ScreenPosition`) (`local.__WorldContext`)) true)
              (`KismetArrayLibrary.Array_Add` (`/Game/Smartphone/BP/DeviceComponents/BP_SmartphoneComponent.Notifications` (`local.SmartphoneCompRef`)) (make `/Game/Smartphone/Structures/Notification_Struct` (`local.App`) (`local.Title`) (`local.NotifText`)))
              (return (`local.CreatedNotification`)))
            (:`else`)))))))

(fn `SendTextMessage`
  (params (PawnRef :type "Pawn Object Reference") (`(Optional) DialogueName` :type Text) (From :type Text) (Text :type Text))
  (locals (SmartphoneRef :type "/Game/Smartphone/BP/DeviceComponents/BP_SmartphoneComponent Object Reference") (CurrentDialoguesList :type "Array of /Game/Smartphone/Structures/MsgDialogues_Struct Structure") (TargetDialogue :type Integer))
  (bind __optional__dialoguename (`local.(Optional) DialogueName`))
  (bind (_output_dialoguetitle _output_messages) (break `/Game/Smartphone/Structures/MsgDialogues_Struct` (`|GetArrayItem` (`local.CurrentDIaloguesList`) (`local.TargetDialogue`))))
  (bind _output_get (set `local.SmartphoneRef` (`Actor.GetComponentByClass` PawnRef "/Game/Smartphone/BP/DeviceComponents/BP_SmartphoneComponent.BP_SmartphoneComponent_C")))
  (`/Engine/EditorBlueprintResources/StandardMacros.IsValid` _output_get
    (:`Is Valid`
      (set `local.CurrentDialoguesList` (`/Game/Smartphone/BP/DeviceComponents/BP_SmartphoneComponent.Messages` _output_get))
      (`|ExecutionSequence`
        (:`then_0`
          (for (_array_element _array_index) (`local.CurrentDIaloguesList`)
            (if (`KismetTextLibrary.EqualEqual_TextText` (`.DialogueTitle_5_5B57D4C84E33226E477F3BB1C601BB81` (break `/Game/Smartphone/Structures/MsgDialogues_Struct` _array_element)) (select `bool` (`KismetTextLibrary.TextIsEmpty` (`local.(Optional) DialogueName`)) :`false` (`local.(Optional) DialogueName`) :`true` (`local.From`)))
              (set `local.TargetDialogue` _array_index)
              (break))))
        (:`then_1`
          (if (== (`local.TargetDialogue`) -1)
            (`KismetArrayLibrary.Array_Add` (`local.CurrentDIaloguesList`) (make `/Game/Smartphone/Structures/MsgDialogues_Struct` (select `bool` (`KismetTextLibrary.TextIsEmpty` __optional__dialoguename) :`false` __optional__dialoguename :`true` (`local.From`)) (`|MakeArray` (make `/Game/Smartphone/Structures/PhoneMsg_Struct` (`local.From`) (`local.Text`) false false) :!type "/Game/Smartphone/Structures/PhoneMsg_Struct Structure")))
            (else
              (`KismetArrayLibrary.Array_Add` _output_messages (make `/Game/Smartphone/Structures/PhoneMsg_Struct` (`local.From`) (`local.Text`) false false)))))
        (:`then_2`
          (bind _asplayer_controller (cast `PlayerController` (`Pawn.GetController` (`local.PawnRef`))))
          (`self.SendNotification` _asplayer_controller (`local.From`) (`local.Text`) (make `/Game/Smartphone/Structures/SmartphoneApp_Struct` "Messages" "/Game/Smartphone/Texture/Icon/T_Messages_icon.T_Messages_icon" "/Game/Smartphone/UMG/DevicesBases/PhoneApps/Messages/UMG_SP_Messages.UMG_SP_Messages_C") (`local.PawnRef`)))
        (:`then_3`
          (bind _currentdevice (`/Game/Smartphone/BP/DeviceComponents/BP_DeviceComponent.CurrentDevice` (`local.SmartphoneRef`))
            (:`then`
              (bind _currentumg (`/Game/Smartphone/BP/BP_DeviceActor.CurrentUMG` _currentdevice)
                (:`then`
                  (bind _appreference (message `/Game/Smartphone/BP/BP_DevicesInterface.GetCurrentActiveApp` _currentumg))
                  (bind _asumg_sp_messages (cast `/Game/Smartphone/UMG/DevicesBases/PhoneApps/Messages/UMG_SP_Messages` _appreference))
                  (`/Game/Smartphone/UMG/DevicesBases/PhoneApps/Messages/UMG_SP_Messages.UpdatePreviews` _asumg_sp_messages))
                (:`else`)))
            (:`else`)))
        (:`then_4`
          (set `/Game/Smartphone/BP/DeviceComponents/BP_SmartphoneComponent.Messages` (`local.CurrentDialoguesList`) (`local.SmartphoneRef`)))))))