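; Pawn component that manages a usable device such as a smartphone, spawning it attached to a socket or itself and finishing its use through server-to-all events.
; It relays first-person state to the device and a tagged anim sub-instance, sets navigation mode, and creates an on-screen widget.
; It also handles timer-based battery charging and playlist audio with pause, wrapping track switching and restart-or-previous logic; song completion only prints a message.
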(event `self.ReceiveBeginPlay`
  (`|ExecutionSequence`
    (:`then_0`
      (`self.AnimationBP_Ref`
        (:`then`)
        (:`else`
          (bind _returnvalue (`self.GetAnimBP`))
          (set `self.AnimationBP_Ref` _returnvalue))))
    (:`then_1`
      (bind _asplayer_controller (`self.GetController`))
      (bind _returnvalue_2 (`|CreateWidget` "/Game/Smartphone/UMG/UMG_OnScreenWidgets.UMG_OnScreenWidgets_C" _asplayer_controller))
      (bind _output_get (set `self.OnScreenWidgets` _returnvalue_2))
      (`UserWidget.AddToViewport` _output_get 0)
      (bind _asplayer_controller_2 (`self.GetController`))
      (set `self.PC` _asplayer_controller_2))))

(event `self.ReceiveTick`
  (params (DeltaSeconds :type "Float (single-precision)")))

(event `On Activate Device`
  (`|ExecutionSequence`
    (:`then_0`
      (`self.Server_SpawnDevice`))
    (:`then_1`
      (`self.UpdateFirstPerson` (`self.IsInFP`)))))

(event `All_SpawnDevice`
  ;[1 1 1] Start using the device
  (`self.CurrentDevice`
    (:`then`
      ;[1 1 1] In case we're already using the device, just update the visual stuff
      (`/Game/Smartphone/BP/BP_DeviceActor.SetEnableUI` (`self.CurrentDevice`) (`self.SpawnDeviceWithUI`) true)
      (`/Game/Smartphone/BP/BP_DeviceActor.SetEnableAnimations` (`self.CurrentDevice`) (`self.SpawnDeviceWithAnimations`) true))
    (:`else`
      (bind _returnvalue (`|SpawnActorFromClass` (`self.DeviceClass`) (`self.K2_GetComponentToWorld`) "AlwaysSpawn" "OverrideRootScale" (`self.GetOwner`) (not (`self.ControlModeMouse`)) self (`self.SpawnDeviceWithUI`) (`self.SpawnDeviceWithAnimations`) null))
      (set `self.CurrentDevice` _returnvalue)
      (if (!= (`self.GetAttachSocketName`) "None")
        (`Actor.K2_AttachToComponent` (`self.CurrentDevice`) (`self.GetAttachParent`) (`self.GetAttachSocketName`) "SnapToTarget" "SnapToTarget" "SnapToTarget" true)
        (else
          (`Actor.K2_AttachToComponent` (`self.CurrentDevice`) self "None" "KeepRelative" "KeepRelative" "SnapToTarget" true)
          (`self.ResetRelativeTransform` (`/Game/Smartphone/BP/BP_DeviceActor.DefaultSceneRoot` (`self.CurrentDevice`))))))))

(event `Server_SpawnDevice`
  ;[1 1 1] Start using the device
  (`self.All_SpawnDevice`))

(event `self.UpdateFirstPerson`
  (params (IsInFP :type Boolean))
  ;[1 1 1] Toggle first person mode
  (`self.Client_UpdateFP` IsInFP))

(event `Client_UpdateFP`
  (params (IsInFP :type Boolean))
  ;[1 1 1] Toggle first person mode
  (set `self.IsInFP` IsInFP)
  (bind _animationbp_ref (`self.AnimationBP_Ref`)
    (:`then`
      (message `/Game/Smartphone/BP/BP_DevicesInterface.UpdateFirstPerson` _animationbp_ref (`self.IsInFP`)))
    (:`else`
      _))
  (bind _currentdevice (`self.CurrentDevice`)
    (:`then`
      (`self.UpdateFirstPerson` _currentdevice (`self.IsInFP`)))
    (:`else`)))

(event `self.FinishUsingDevice`
  ;[1 1 1] Finish usage
  (`self.CurrentDevice`
    (:`then`
      (`self.Server_RemoveDevice`))
    (:`else`)))

(event `Server_RemoveDevice`
  ;[1 1 1] Finish usage
  (`self.All_RemoveDevice`))

(event `All_RemoveDevice`
  ;[1 1 1] Finish usage
  (bind _currentdevice (`self.CurrentDevice`)
    (:`then`
      (message `/Game/Smartphone/BP/BP_DevicesInterface.FinishUsingDevice` _currentdevice))
    (:`else`)))

(event `self.SetDeviceCharging`
  (params (NewChargingValue :type Boolean))
  (bind _output_get (set `self.IsCharging` NewChargingValue))
  (if _output_get
    (bind _currentdevice (`self.CurrentDevice`)
      (:`then`
        (bind _currentumg (`/Game/Smartphone/BP/BP_DeviceActor.CurrentUMG` _currentdevice)
          (:`then`
            (bind _devicewidget (`/Game/Smartphone/UMG/UMG_OnScreenDevice.DeviceWidget` _currentumg)
              (:`then`
                (message `/Game/Smartphone/BP/BP_DevicesInterface.SetDeviceCharging` _devicewidget (`self.IsCharging`)))
              (:`else`)))
          (:`else`)))
      (:`else`
        ;[1 1 1] We should be able to charge the phone even when it is not in use
        (bind _returnvalue (`KismetSystemLibrary.K2_SetTimerDelegate` (delegate `BatteryCharge`) 1.0 true))
        (set `self.ChargingTimer` _returnvalue)))
    (else
      (`KismetSystemLibrary.K2_ClearAndInvalidateTimerHandle` (`self.ChargingTimer`)))))

(event `BatteryCharge`
  ;[1 1 1] We should be able to charge the phone even when it is not in use
  (`self.CurrentDevice`
    (:`then`
      (`KismetSystemLibrary.K2_ClearAndInvalidateTimerHandle` (`self.ChargingTimer`))
      (set `self.CurrentBatteryLevel` (+ (`self.CurrentBatteryLevel`) (`self.ChargingPerSecond`))))
    (:`else`)))

(fn `Animation_DeviceInitialized`
  (returns (AnimationStartupLaunched :type Boolean) (AnimationLen :type "Float (double-precision)"))
  (return false 0.0))

(fn `Animation_FinishedUsingDevice`
  (returns (PlayingFinishAnimation :type Boolean) (FinishAnimDuration :type "Float (double-precision)"))
  (return false 0.0))

(fn `GetAnimBP`
  (returns (ReturnValue :type "AnimInstance Object Reference"))
  (bind _asskeletal_mesh_component (cast `SkeletalMeshComponent` (`self.GetAttachParent`)))
  (return (`AnimInstance.GetSubInstanceByTag` (`SkeletalMeshComponent.GetAnimInstance` _asskeletal_mesh_component) (`self.AnimationBP_Tag`))))

(fn `GetCurrentActiveApp`
  (returns (AppReference :type "UserWidget Object Reference"))
  (return null))

(fn `GetDevice`
  (params (StartDeviceWithUI :type Boolean :default true) (StartDeviceWithAnimations :type Boolean :default true))
  (set `self.SpawnDeviceWithUI` StartDeviceWithUI)
  (set `self.SpawnDeviceWithAnimations` StartDeviceWithAnimations)
  (`self.On Activate Device`))

(fn `PlayCurrentSong`
  (`|ExecutionSequence`
    (:`then_0`
      (bind _currentaudio (`self.CurrentAudio`)
        (:`then`
          (bind _returnvalue (`AudioComponent.IsPlaying` _currentaudio))
          (if _returnvalue
            (if (`KismetSystemLibrary.K2_IsTimerPausedHandle` (`self.CurrentMusicTimer`))
              (`AudioComponent.SetPaused` (`self.CurrentAudio`) false)
              (`KismetSystemLibrary.K2_UnPauseTimerHandle` (`self.CurrentMusicTimer`))
              (else
                (`AudioComponent.SetPaused` (`self.CurrentAudio`) true)
                (`KismetSystemLibrary.K2_PauseTimerHandle` (`self.CurrentMusicTimer`))))
            (else
              (`AudioComponent.Stop` (`self.CurrentAudio`))
              (`AudioComponent.SetSound` (`self.CurrentAudio`) (`self.CurrentSongSound`))
              (`AudioComponent.Play` (`self.CurrentAudio`) 0.0)
              (`self.ReinitTimer`))))
        (:`else`
          (bind _returnvalue_2 (`GameplayStatics.CreateSound2D` (`self.CurrentSongSound`) 1.0 1.0 0.0 null))
          (bind _output_get (set `self.CurrentAudio` _returnvalue_2))
          (`self.SetActive` _output_get true false)
          (`AudioComponent.Play` _output_get 0.0)
          (`self.ReinitTimer`))))
    (:`then_1`
      (setmembers `/Game/Smartphone/Structures/CurrentPlaylistInfo_Struct` :`StructRef` (`self.CurrentPlaylistInfo`) :`IsPaused` (not _returnvalue)))))

(fn `SetInputModeScroll`
  (params (ControlModeScroll :type Boolean))
  (set `self.ControlModeMouse` (not ControlModeScroll))
  (bind _currentdevice (`self.CurrentDevice`)
    (:`then`
      (set `/Game/Smartphone/BP/BP_DeviceActor.NavigationControls` ControlModeScroll _currentdevice))
    (:`else`)))

(fn `SongFinish`
  (`KismetSystemLibrary.PrintString` "Song finished"))

(fn `SwitchTrack`
  (params (PreviousTrack :type Boolean))
  (locals (TargetIndex :type Integer :default 0))
  (bind (_currentplaylistinfo_currplaylistinfo _currentplaylistinfo_currsongindex) (break `/Game/Smartphone/Structures/CurrentPlaylistInfo_Struct` (`self.CurrentPlaylistInfo`)))
  (bind (_currentplaylistinfo_currplaylistinfo_2 _currentplaylistinfo_currsongindex_2) (break `/Game/Smartphone/Structures/CurrentPlaylistInfo_Struct` (`self.CurrentPlaylistInfo`)))
  (bind _returnvalue (- _currentplaylistinfo_currsongindex 1))
  (bind _returnvalue_2 (+ _currentplaylistinfo_currsongindex_2 1))
  (`self.CurrentAudio`
    (:`then`
      (if PreviousTrack
        (if (`KismetSystemLibrary.K2_IsTimerActiveHandle` (`self.CurrentMusicTimer`))
          (if (< (`KismetSystemLibrary.K2_GetTimerElapsedTimeHandle` (`self.CurrentMusicTimer`)) 3.0)
            (set `local.TargetIndex` (`KismetMathLibrary.SelectInt` (`KismetMathLibrary.SelectInt` (`KismetArrayLibrary.Array_LastIndex` (`.Songs_7_E5AB5D1C415E33F51844C4987DAD85EB` (break `/Game/Smartphone/Structures/MusicPlaylist_Struct` _currentplaylistinfo_currplaylistinfo))) _returnvalue (< _returnvalue 0)) (`KismetMathLibrary.SelectInt` 0 _returnvalue_2 (> _returnvalue_2 (`KismetArrayLibrary.Array_LastIndex` (`.Songs_7_E5AB5D1C415E33F51844C4987DAD85EB` (break `/Game/Smartphone/Structures/MusicPlaylist_Struct` _currentplaylistinfo_currplaylistinfo_2))))) (`local.PreviousTrack`)) :!label _label)
            (setmembers `/Game/Smartphone/Structures/CurrentPlaylistInfo_Struct` :`StructRef` (`self.CurrentPlaylistInfo`) :`CurrSongIndex` (`local.TargetIndex`))
            (bind _currentaudio (`self.CurrentAudio`)
              (:`then`
                (`AudioComponent.Stop` _currentaudio)
                (`AudioComponent.SetSound` _currentaudio (`self.CurrentSongSound`))
                (`self.ReinitTimer`)
                (`AudioComponent.Play` _currentaudio 0.0))
              (:`else`))
            (else
              (`self.RestartCurrSong`)))
          (else
            (goto _label)))
        (else
          (goto _label))))
    (:`else`)))

(fn `UpdateWidgetVisibility`
  (bind _currentdevice (`self.CurrentDevice`)
    (:`then`)
    (:`else`)))