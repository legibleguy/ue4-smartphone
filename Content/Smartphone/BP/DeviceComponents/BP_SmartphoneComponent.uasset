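; Smartphone device component that holds a character's phone state: number, contacts, settings, wallpaper and songs.
; BeginPlay loads songs from a playlist data table, generates a random number if none is set and tags the owner with it.
; Calls reject if already speaking, otherwise store the caller, relay speaking state through REP/ALL events and drive talking animations.
; Tick pushes brightness to the screen material; notification handling and track debug keys are disconnected.
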(event `self.ReceiveBeginPlay`
  (`parent.ReceiveBeginPlay`)
  (`|ExecutionSequence`
    (:`then_0`
      (bind _playliststable (`self.PlaylistsTable`)
        (:`then`
          (bind _outrownames (`DataTableFunctionLibrary.GetDataTableRowNames` _playliststable))
          (for _array_element _outrownames
            (bind _returnvalue (`|GetDataTableRow` _playliststable _array_element)
              (:`then`
                (`KismetArrayLibrary.Array_Add` (`self.SongsOnThePhone`) _returnvalue)))))
        (:`else`)))
    (:`then_1`
      (if (not (!= (`self.PhoneNumber`) "None"))
        (`self.GenerateRandomNumber`))
      (`self.AddNumberToChar`))))

(event `self.ReceiveTick`
  (params (DeltaSeconds :type "Float (single-precision)"))
  (bind (_phonesettings_uselowpowermode _phonesettings_showbatterypercent _phonesettings_brightness) (break `/Game/Smartphone/Structures/PhoneSettings_Struct` (`self.PhoneSettings`)))
  (`parent.ReceiveTick` DeltaSeconds)
  (`|ExecutionSequence`
    (:`then_0`
      (bind _currentdevice (`self.CurrentDevice`)
        (:`then`
          (bind _screenmaterial (`/Game/Smartphone/BP/BP_DeviceActor.GetScreenMat` _currentdevice))
          (`/Engine/EditorBlueprintResources/StandardMacros.IsValid` _screenmaterial
            (:`Is Valid`
              (`MaterialInstanceDynamic.SetScalarParameterValue` _screenmaterial "Brightness" _phonesettings_brightness))))
        (:`else`)))))

(event `self.All_SpawnDevice`
  (`parent.All_SpawnDevice`))

(event `GenerateRandomNumber`
  (bind _returnvalue (`KismetStringLibrary.Conv_IntToString` (`KismetMathLibrary.RandomInteger` 9)))
  (for _ (range 9)
    (if (`KismetStringLibrary.IsNumeric` (`KismetStringLibrary.Conv_NameToString` (`self.PhoneNumber`)))
      (set `self.PhoneNumber` (`KismetStringLibrary.Conv_StringToName` (`KismetStringLibrary.Concat_StrStr` (`KismetStringLibrary.Conv_NameToString` (`self.PhoneNumber`)) _returnvalue)))
      (else
        (set `self.PhoneNumber` (`KismetStringLibrary.Conv_StringToName` _returnvalue)))))
  (`self.ClientRememberNum` (`KismetSystemLibrary.MakeLiteralName` (`self.PhoneNumber`))))

(event `self.Server_SpawnDevice`
  (`parent.Server_SpawnDevice`)
  (`self.TryToInteractWithNotification`))

(event `ClientRememberNum`
  (params (NewItem :type "Name (by ref)"))
  (set `self.PhoneNumber` NewItem))

(event `AddNumberToChar`
  (`KismetArrayLibrary.Array_Add` (`Actor.Tags` (`self.GetOwner`)) (`self.PhoneNumber`)))

(event `self.BreakCall`
  (`|ExecutionSequence`
    (:`then_0`
      (bind _animationbp_ref (`self.AnimationBP_Ref`)
        (:`then`
          (message `/Game/Smartphone/BP/BP_SmartphoneInterface.Animation_QuitSpeakingOnThePhone` _animationbp_ref))
        (:`else`)))
    (:`then_1`
      (bind _aspawn (cast `Pawn` (`self.GetOwner`))
        (:`then`
          (if (not (`Pawn.IsPlayerControlled` _aspawn))
            (`self.FinishUsingDevice` :!label _label)))
        (:`CastFailed`
          (goto _label))))
    (:`then_2`
      (`self.REP_UpdatePhoneSpeakingValue` false))))

(event `CallReceiveEvent`
  (params (From :type "/Game/Smartphone/BP/DeviceComponents/BP_SmartphoneComponent Object Reference"))
  (`/Game/Smartphone/BP/BP_DeviceActor.PC` (`self.CurrentDevice`)
    (:`then`)
    (:`else`
      (`KismetSystemLibrary.PrintString` "AI received call"))))

(event `REP_UpdatePhoneSpeakingValue`
  (params (NewVal :type Boolean))
  (`self.ALL_UpdatePhoneSpeakingValue` NewVal))

(event `ALL_UpdatePhoneSpeakingValue`
  (params (NewVal :type Boolean))
  (set `self.SpeakingOnThePhone` NewVal))

(event `CallMadeEvent`
  (params (To :type "/Game/Smartphone/BP/DeviceComponents/BP_SmartphoneComponent Object Reference"))
  (`self.REPL_CallMade` To))

(event `REPL_CallMade`
  (params (To :type "/Game/Smartphone/BP/DeviceComponents/BP_SmartphoneComponent Object Reference"))
  (`|ExecutionSequence`
    (:`then_0`
      (bind _success_ (`self.CallMade` To))
      (if _success_
        (bind _animationbp_ref (`/Game/Smartphone/BP/DeviceComponents/BP_DeviceComponent.AnimationBP_Ref` To)
          (:`then`
            (message `/Game/Smartphone/BP/BP_SmartphoneInterface.Animation_SpeakingOnThePhone` _animationbp_ref))
          (:`else`))))
    (:`then_1`
      (`self.ALL_CallMade` To))))

(event `ALL_CallMade`
  (params (To :type "/Game/Smartphone/BP/DeviceComponents/BP_SmartphoneComponent Object Reference"))
  (bind _success_ (`self.CallMade` To))
  (if _success_
    (bind _animationbp_ref (`/Game/Smartphone/BP/DeviceComponents/BP_DeviceComponent.AnimationBP_Ref` To)
      (:`then`
        (message `/Game/Smartphone/BP/BP_SmartphoneInterface.Animation_SpeakingOnThePhone` _animationbp_ref))
      (:`else`))))

(fn `AddNumber`
  (params (NewContact :type "/Game/Smartphone/BP/DeviceData/PhoneContact Structure (by ref)"))
  (`KismetArrayLibrary.Array_Add` (`self.Phone Contacts`) NewContact))

(fn `CallMade`
  (params (To :type "/Game/Smartphone/BP/DeviceComponents/BP_SmartphoneComponent Object Reference"))
  (returns (`Success?` :type Boolean))
  (`self.InitPhoneCall`
    (:`Already speaking`
      (return false))
    (:`All Good`
      (`self.On Activate Device`)
      (set `self.Caller` To)
      (return true))))

(fn `CallReceive`
  (params (From :type "/Game/Smartphone/BP/DeviceComponents/BP_SmartphoneComponent Object Reference"))
  (returns (NotAvailable :type Boolean))
  (`self.InitPhoneCall`
    (:`Already speaking`
      (return true))
    (:`All Good`
      (set `self.Caller` From)
      (return false))))

(fn `CameraUpdateX`
  (params (`X Val` :type "Float (double-precision)"))
  (returns (CurrValue :type "Float (double-precision)"))
  (return 0.0))

(fn `CameraUpdateY`
  (params (`Y Val` :type "Float (double-precision)"))
  (returns (CurrValue :type "Float (double-precision)"))
  (return 0.0))

(fn `GetCurrentScreenshots`
  (returns (AllScreens :type "Array of Texture2D Object Reference"))
  (return))

(fn `GetNotesArray`
  (returns (ArrayExists :type Boolean) (OutNotes :type "Array of /Game/Smartphone/BP/DeviceData/Note Structure"))
  (return false (`self.NotesOnTheDevice`)))

(fn `GetNotifBarTemporaryColors`
  (returns (ShouldUpdate :type Boolean) (TempDefault :type "LinearColor Structure") (TempHover :type "LinearColor Structure") (TempPressed :type "LinearColor Structure"))
  (return false))

(fn `GetPhoneWidgets`
  (returns (`Out Widgets` :type "Array of UserWidget Class Reference"))
  (return (`self.AppWidgets`)))

(fn `MiddleMousePress`
  (returns (ActionTaken :type Boolean))
  (return false))

(fn `RequestPhoneSettings`
  (returns (OutSettings :type "/Game/Smartphone/Structures/PhoneSettings_Struct Structure"))
  (return (`self.PhoneSettings`)))

(fn `RightAltPress`
  (returns (ActionTaken :type Boolean))
  (return false))

(fn `TryToInteractWithNotification`
  (locals (AllNotif :type "Array of /Game/Smartphone/UMG/DevicesBases/SmartphoneFeatures/NotifCenter/UMG_Notification Object Reference")))

(fn `UpdateCurrentWallpaper`
  (locals (Target :type "MaterialInterface Object Reference"))
  (bind (_phonesettings_uselowpowermode _phonesettings_showbatterypercent _phonesettings_brightness _phonesettings_cameraresolutionmultiplier _phonesettings_wallpapermat) (break `/Game/Smartphone/Structures/PhoneSettings_Struct` (`self.PhoneSettings`)))
  (bind (_allwallpapers _selectedwallpaper) (break `/Game/Smartphone/Structures/DeviceWallpaper_Struct` _phonesettings_wallpapermat))
  (bind _output_get (set `local.Target` (`|GetArrayItem` _allwallpapers _selectedwallpaper)))
  (`/Engine/EditorBlueprintResources/StandardMacros.IsValid` _output_get
    (:`Is Valid`
      (bind _currentdevice (`self.CurrentDevice`)
        (:`then`
          (bind _currentumg (`/Game/Smartphone/BP/BP_DeviceActor.CurrentUMG` _currentdevice)
            (:`then`
              (bind _devicewidget (`/Game/Smartphone/UMG/UMG_OnScreenDevice.DeviceWidget` _currentumg)
                (:`then`
                  (message `/Game/Smartphone/BP/BP_SmartphoneInterface.SetWallpaper` _devicewidget (`local.Target`)))
                (:`else`)))
            (:`else`)))
        (:`else`)))))