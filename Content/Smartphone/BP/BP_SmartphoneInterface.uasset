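; BP_SmartphoneInterface is a Blueprint Interface defining the contract for an in-game smartphone.
; Its stub functions cover mouse and key input, calls with speaking animations, and camera app control including photo capture, grid, look and tilt.
; Further functions expose phone widgets, screenshots, settings, wallpaper and temporary notification bar colors.
; It holds no logic, so implementers supply the behavior.
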(fn `AddCameraTilt`
  (params (Value :type "Float (double-precision)")))

(fn `Animation_QuitSpeakingOnThePhone`)

(fn `Animation_SpeakingOnThePhone`)

(fn `BreakCall`)

(fn `CallMade`
  (params (To :type "/Game/Smartphone/BP/DeviceComponents/BP_SmartphoneComponent Object Reference"))
  (returns (`Success?` :type Boolean))
  (return false))

(fn `CallReceive`
  (params (From :type "/Game/Smartphone/BP/DeviceComponents/BP_SmartphoneComponent Object Reference"))
  (returns (NotAvailable :type Boolean))
  (return false))

(fn `CameraUpdateX`
  (params (`X Val` :type "Float (double-precision)"))
  (returns (CurrValue :type "Float (double-precision)"))
  (return 0.0))

(fn `CameraUpdateY`
  (params (`Y Val` :type "Float (double-precision)"))
  (returns (CurrValue :type "Float (double-precision)"))
  (return 0.0))

(fn `EnableFrontCamera`)

(fn `EnableMainCamera`)

(fn `GetCurrentScreenshots`
  (returns (AllScreens :type "Array of Texture2D Object Reference"))
  (return))

(fn `GetNotifBarTemporaryColors`
  (returns (ShouldUpdate :type Boolean) (TempDefault :type "LinearColor Structure") (TempHover :type "LinearColor Structure") (TempPressed :type "LinearColor Structure"))
  (return false))

(fn `GetPhoneWidgets`
  (returns (`Out Widgets` :type "Array of UserWidget Class Reference"))
  (return))

(fn `MiddleMousePress`
  (returns (ActionTaken :type Boolean))
  (return false))

(fn `MiddleMouseRelease`)

(fn `OnCameraAppStarted`
  (params (`Camera Widget` :type "UserWidget Object Reference")))

(fn `OnDisableCamera`
  (params (`Use Controller Yaw` :type Boolean) (`Orient Rotation` :type Boolean)))

(fn `OnPhoneSettingsChanged`
  (params (CurrentSettings :type "/Game/Smartphone/Structures/PhoneSettings_Struct Structure")))

(fn `OnTakePhoto`)

(fn `RequestPhoneSettings`
  (returns (OutSettings :type "/Game/Smartphone/Structures/PhoneSettings_Struct Structure"))
  (return))

(fn `RightAltPress`
  (returns (ActionTaken :type Boolean))
  (return false))

(fn `RightAltRelease`)

(fn `SetWallpaper`
  (params (WallpaperAsset :type "MaterialInterface Object Reference")))

(fn `StopTakingPhoto`)

(fn `ToggleCameraGrid`)