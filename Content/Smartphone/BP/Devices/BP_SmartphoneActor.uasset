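; Handheld smartphone device actor with a working main/front camera and extra battery drain from app use, brightness and power mode.
; Timers sync mesh visibility and destruction to the midpoint of the pawn's get and put-away animations.
; Camera mode blends the view to the phone, sends rotation and tilt to the pawn's animation Blueprint, and zooms via FOV.
; Photos use the HighResShot console command and are reloaded from disk as textures.
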(event `self.ReceiveBeginPlay`
  (`parent.ReceiveBeginPlay`))

(event `self.ReceiveTick`
  (params (DeltaSeconds :type "Float (single-precision)"))
  (`parent.ReceiveTick` DeltaSeconds)
  (if (`self.UsingCamera`)
    (`self.CameraUpdate` DeltaSeconds)))

(event `self.Animation Init`
  ;[1 1 1] This setup will show smartphone only after character reaches the pocket
  (if (`self.EnableAnimations`)
    (bind _returnvalue (`self.Pawn-GetAnimationBlueprint`))
    (`/Engine/EditorBlueprintResources/StandardMacros.IsValid` _returnvalue
      (:`Is Valid`
        (bind (_animationstartuplaunched _animationlen) (message `/Game/Smartphone/BP/BP_DevicesInterface.Animation_DeviceInitialized` _returnvalue))
        (if _animationstartuplaunched
          (`SceneComponent.SetVisibility` (`self.PhoneMesh`) false false)
          (`KismetSystemLibrary.K2_SetTimerDelegate` (delegate `VisibilityReset`) (/ _animationlen 2.0)))))
    (else
      (bind _returnvalue_2 (`self.Pawn-GetAnimationBlueprint`))
      (`/Engine/EditorBlueprintResources/StandardMacros.IsValid` _returnvalue_2
        (:`Is Valid`
          (message `/Game/Smartphone/BP/BP_DevicesInterface.Animation_FinishedUsingDevice` _returnvalue_2))))))

(event `VisibilityReset`
  ;[1 1 1] This setup will show smartphone only after character reaches the pocket
  (`SceneComponent.SetVisibility` (`self.PhoneMesh`) true false))

(event `/Game/Smartphone/BP/BP_DevicesInterface.FinishUsingDevice`
  ;[1 1 1] Just like with the startup, this will allow us to completely destroy the device actor only halfway through the finish animation
  (bind _returnvalue (`self.Pawn-GetAnimationBlueprint`))
  (bind (_playingfinishanimation _finishanimduration) (message `/Game/Smartphone/BP/BP_DevicesInterface.Animation_FinishedUsingDevice` _returnvalue))
  (if _playingfinishanimation
    (`KismetSystemLibrary.K2_SetTimerDelegate` (delegate `CompleteDestruction`) (/ _finishanimduration 2.0))
    (else
      (`self.CompleteDestruction`))))

(event `CompleteDestruction`
  ;[1 1 1] Just like with the startup, this will allow us to completely destroy the device actor only halfway through the finish animation
  (`self.K2_DestroyActor`))

(event `Key|LeftMouseButton`
  (params (Key :type "Key Structure"))
  (bind (_returnvalue_x _returnvalue_y) (`KismetMathLibrary.BreakVector2D` (* (`WidgetLayoutLibrary.GetViewportSize`) (`self.PhotoResolutionMultiply`))))
  ;[1 1 1] You may replace this with your own input actions
  (:`Pressed`
    (`self.Is Using Camera?` :!label _label
      (:`Is Valid`
        (set `self.CameraButtonDown` true))))
  (:`Released`
    (`self.Is Using Camera?` :!label _label_2
      (:`Is Valid`
        (if (`self.CameraButtonDown`)
          (bind _outsettings (message `/Game/Smartphone/BP/BP_SmartphoneInterface.RequestPhoneSettings` (`self.ComponentReference`)))
          (set `self.PhotoResolutionMultiply` (`.CameraResolutionMultiplier_9_BC22CD224F1941E3BB1A5785E566B8E2` (break `/Game/Smartphone/Structures/PhoneSettings_Struct` _outsettings)))
          (`KismetSystemLibrary.ExecuteConsoleCommand` (`KismetStringLibrary.Concat_StrStr` "HighResShot " (`KismetStringLibrary.Concat_StrStr` (`KismetStringLibrary.Conv_IntToString` (`KismetMathLibrary.FTrunc` _returnvalue_x)) "x" (`KismetStringLibrary.Conv_IntToString` (`KismetMathLibrary.FTrunc` _returnvalue_y)))) (`self.GetPC`))
          (set `self.CameraButtonDown` false)
          (message `/Game/Smartphone/BP/BP_SmartphoneInterface.OnTakePhoto` (`self.CurrentCamUMG`)))))))

(event `Key|Gamepad_FaceButton_Bottom`
  (params (Key :type "Key Structure"))
  ;[1 1 1] You may replace this with your own input actions
  (:`Pressed`
    (goto _label))
  (:`Released`
    (goto _label_2)))

(event `InputAction|CameraTiltToggle`
  (params (Key :type "Key Structure"))
  (bind _asplayer_controller (`self.GetPC`))
  (:`Pressed`
    (set `self.IsTiltingCamera` true)
    (set `PlayerController.InputYawScale` 0.0 _asplayer_controller)
    (set `PlayerController.InputPitchScale` 0.0 _asplayer_controller))
  (:`Released`
    (set `self.IsTiltingCamera` false)
    (set `PlayerController.InputYawScale` 2.5 _asplayer_controller)
    (set `PlayerController.InputPitchScale` 2.5 _asplayer_controller)))

(event `self.EnableMainCamera`
  (set `self.UsingFrontCamera` false)
  (`|ExecutionSequence`
    (:`then_0`
      (`|ExecutionSequence`
        (:`then_0`
          (bind _returnvalue (`self.Pawn-GetAnimationBlueprint`))
          (`/Engine/EditorBlueprintResources/StandardMacros.IsValid` _returnvalue
            (:`Is Valid`
              (message `/Game/Smartphone/BP/BP_SmartphoneInterface.EnableFrontCamera` _returnvalue))))
        (:`then_1`
          (`ActorComponent.SetActive` (`self.FrontCamera`) false false)
          (`ActorComponent.SetActive` (`self.MainCamera`) true false))))
    (:`then_1`
      (`PlayerController.SetViewTargetWithBlend` (`self.GetPC`) self (`self.CameraBlendTime`) "VTBlend_Cubic" 1.34 false :!label _label_3)
      (set `self.UsingCamera` false)
      (`KismetSystemLibrary.K2_SetTimerDelegate` (delegate `CameraBlendFinished`) (`self.CameraBlendTime`)))))

(event `CameraBlendFinished`
  (set `self.UsingCamera` true))

(event `self.EnableFrontCamera`
  (set `self.UsingFrontCamera` true)
  (`|ExecutionSequence`
    (:`then_0`
      (`|ExecutionSequence`
        (:`then_0`
          (bind _returnvalue (`self.Pawn-GetAnimationBlueprint`))
          (`/Engine/EditorBlueprintResources/StandardMacros.IsValid` _returnvalue
            (:`Is Valid`
              (message `/Game/Smartphone/BP/BP_SmartphoneInterface.EnableMainCamera` _returnvalue))))
        (:`then_1`
          (`ActorComponent.SetActive` (`self.MainCamera`) false false)
          (`ActorComponent.SetActive` (`self.FrontCamera`) true false))))
    (:`then_1`
      (goto _label_3))))

(event `InputAction|CameraToggle`
  (params (Key :type "Key Structure"))
  (:`Pressed`
    (if (`self.UsingCamera`)
      (if (`ActorComponent.IsActive` (`self.FrontCamera`))
        (`self.EnableMainCamera`)
        (else
          (`self.EnableFrontCamera`))))))

(event `CameraUpdate`
  (params (Delta :type "Float (double-precision)"))
  (bind _maincamera (`self.MainCamera`))
  (bind (_relativerotation_roll _relativerotation_pitch _relativerotation_yaw) (`KismetMathLibrary.BreakRotator` (`SceneComponent.RelativeRotation` (`self.PhoneMesh`))))
  (bind (_relativerotation_roll_2 _relativerotation_pitch_2) (`KismetMathLibrary.BreakRotator` (`SceneComponent.RelativeRotation` (`self.PhoneMesh`))))
  (bind _returnvalue (select `bool` (`ActorComponent.IsActive` _maincamera) :`false` (`self.FrontCamera`) :`true` _maincamera :!type "CameraComponent Object Reference"))
  (if (`self.ControlsInput`)
    (`|ExecutionSequence`
      (:`then_0`
        (if (`self.IsTiltingCamera`)
          (bind _returnvalue_2 (`self.Pawn-GetAnimationBlueprint`))
          (`/Engine/EditorBlueprintResources/StandardMacros.IsValid` _returnvalue_2
            (:`Is Valid`
              (bind _returnvalue_3 (`self.Pawn-GetAnimationBlueprint`))
              (message `/Game/Smartphone/BP/BP_SmartphoneInterface.AddCameraTilt` _returnvalue_3 (`self.Camera X To Add`)))
            (:`Is Not Valid`
              (`SceneComponent.K2_SetRelativeRotation` (`self.PhoneMesh`) (`KismetMathLibrary.MakeRotator` _relativerotation_roll (`KismetMathLibrary.FClamp` (+ _relativerotation_pitch_2 (* (`self.Camera X To Add`) (`self.TiltScale`))) 1.0 89.0) _relativerotation_yaw) false false)))
          (else
            (bind _returnvalue_4 (`self.Pawn-GetAnimationBlueprint`))
            (message `/Game/Smartphone/BP/BP_SmartphoneInterface.CameraUpdateY` _returnvalue_4 (`self.Camera Y To Add`))
            (bind _currvalue (message `/Game/Smartphone/BP/BP_SmartphoneInterface.CameraUpdateX` _returnvalue_4 (`self.Camera X To Add`)))
            (bind _output_get (set `self.CurrentCameraX` _currvalue))
            (if (> (`KismetMathLibrary.Abs` (+ _output_get (`self.Camera X To Add`))) 90.0)
              (`PlayerController.AddYawInput` (`self.GetPC`) (`self.Camera X To Add`))))))
      (:`then_1`
        (`CameraComponent.SetFieldOfView` _returnvalue (`KismetMathLibrary.FClamp` (+ (`CameraComponent.FieldOfView` _returnvalue) (* (`self.GetInputAxisValue`) (`self.MouseZoomSensitivity`))) 35.0 120.0))))))

(event `self.OnCameraAppStarted`
  (params (`Camera Widget` :type "UserWidget Object Reference"))
  (set `self.CurrentCamUMG` `Camera Widget`))

(event `self.OnDisableCamera`
  (params (`Use Controller Yaw` :type Boolean) (`Orient Rotation` :type Boolean))
  (bind _returnvalue (`self.Pawn-GetAnimationBlueprint`))
  (message `/Game/Smartphone/BP/BP_SmartphoneInterface.OnDisableCamera` _returnvalue false false)
  (set `self.UsingCamera` false)
  (set `self.CurrentCamUMG` null)
  (`PlayerController.SetViewTargetWithBlend` (`self.GetPC`) (`self.GetOwner`) (`self.CameraBlendTime`) "VTBlend_Cubic" 1.34 false))

(fn `AdditionalBatteryConsumption`
  (returns (Out :type "Float (double-precision)"))
  (locals (Add :type "Float (double-precision)" :default 0.0))
  (`|ExecutionSequence`
    (:`then_0`
      (set `local.Add` (`parent.AdditionalBatteryConsumption`)))
    (:`then_1`
      (bind _currentumg (`self.CurrentUMG`)
        (:`then`
          (bind _devicewidget (`/Game/Smartphone/UMG/UMG_OnScreenDevice.DeviceWidget` _currentumg)
            (:`then`
              (bind _appreference (message `/Game/Smartphone/BP/BP_DevicesInterface.GetCurrentActiveApp` _devicewidget))
              (set `local.Add` (+ (* (`self.BatteryConsumptionPerSecond`) (`KismetMathLibrary.SelectFloat` 0.5 0.0 (`KismetSystemLibrary.IsValid` _appreference))) (`local.Add`))))
            (:`else`)))
        (:`else`)))
    (:`then_2`
      (bind _componentreference (`self.ComponentReference`)
        (:`then`
          (bind _outsettings (message `/Game/Smartphone/BP/BP_SmartphoneInterface.RequestPhoneSettings` _componentreference))
          (`|ExecutionSequence`
            (:`then_0`
              (bind (_uselowpowermode _showbatterypercent _brightness) (break `/Game/Smartphone/Structures/PhoneSettings_Struct` _outsettings))
              (set `local.Add` (+ (* (`KismetMathLibrary.Lerp` 0.0 0.45 _brightness) (`self.BatteryConsumptionPerSecond`)) (`local.Add`))))
            (:`then_1`
              (bind _output_get (set `local.Add` (+ (stale _output_get) (* (`KismetMathLibrary.SelectFloat` -0.25 0.0 _uselowpowermode) (`local.Add`))))))))
        (:`else`)))
    (:`then_3`
      (return (`local.Add`)))))

(fn `CallMade`
  (params (To :type "/Game/Smartphone/BP/DeviceComponents/BP_SmartphoneComponent Object Reference"))
  (returns (`Success?` :type Boolean))
  (return false))

(fn `CallReceive`
  (params (From :type "/Game/Smartphone/BP/DeviceComponents/BP_SmartphoneComponent Object Reference"))
  (returns (NotAvailable :type Boolean))
  (return false))

(fn `CameraShot`
  (locals (CurrApp :type "UserWidget Object Reference")))

(fn `CameraUpdateX`
  (params (`X Val` :type "Float (double-precision)"))
  (returns (CurrValue :type "Float (double-precision)"))
  (return 0.0))

(fn `CameraUpdateY`
  (params (`Y Val` :type "Float (double-precision)"))
  (returns (CurrValue :type "Float (double-precision)"))
  (return 0.0))

(fn `GenerateScreenshotName`
  (params (Number :type Integer))
  (returns (ReturnValue :type String))
  (locals (Len :type Integer :default 0) (Out :type String))
  (bind _output_get (set `local.Out` (`KismetStringLibrary.Conv_IntToString` Number)))
  (bind _output_get_2 (set `local.Len` (`KismetStringLibrary.Len` _output_get)))
  (if (>= _output_get_2 5)
    (return (`KismetStringLibrary.Concat_StrStr` (`BlueprintPathsLibrary.ScreenShotDir`) "HighresScreenshot" (`local.Out`) ".png"))
    (else
      (for _ (range 1 (+ (- 5 (`local.Len`)) 1))
        (set `local.Out` (`KismetStringLibrary.Concat_StrStr` "0" (`local.Out`))))
      (return (`KismetStringLibrary.Concat_StrStr` (`BlueprintPathsLibrary.ScreenShotDir`) "HighresScreenshot" (`local.Out`) ".png")))))

(fn `GetCurrentScreenshots`
  (returns (AllScreens :type "Array of Texture2D Object Reference"))
  (locals (OutScreens :type "Array of Texture2D Object Reference") (LastFoundScreenshot :type "Texture2D Object Reference"))
  (for _index (range (`self.MaxScreenshots`))
    (bind _returnvalue (`KismetRenderingLibrary.ImportFileAsTexture2D` (`self.GenerateScreenshotName` _index)))
    (set `local.LastFoundScreenshot` _returnvalue)
    (bind _lastfoundscreenshot (`local.LastFoundScreenshot`)
      (:`then`
        (`KismetArrayLibrary.Array_Add` (`local.OutScreens`) _lastfoundscreenshot))
      (:`else`)))
  (return (`local.OutScreens`)))

(fn `GetNotifBarTemporaryColors`
  (returns (ShouldUpdate :type Boolean) (TempDefault :type "LinearColor Structure") (TempHover :type "LinearColor Structure") (TempPressed :type "LinearColor Structure"))
  (return false))

(fn `GetPhoneWidgets`
  (returns (`Out Widgets` :type "Array of UserWidget Class Reference"))
  (return))

(fn `MiddleMousePress`
  (returns (ActionTaken :type Boolean))
  (return false))

(fn `RequestPhoneSettings`
  (returns (OutSettings :type "/Game/Smartphone/Structures/PhoneSettings_Struct Structure"))
  (return))

(fn `RightAltPress`
  (returns (ActionTaken :type Boolean))
  (return false))

(fn `UserConstructionScript`
  (`parent.UserConstructionScript`)
  (set `self.MainMesh` (`self.PhoneMesh`)))