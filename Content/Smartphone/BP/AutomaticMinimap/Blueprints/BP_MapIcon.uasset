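; BP_MapIcon is a sprite actor that represents its owner on the automatic minimap.
; Each tick it pins itself to Z -99999, nudged by an index parsed from the last character of its display name to prevent overlapping icons.
; Pawn owners rotate the icon by the minimap's rule (fixed, actor, camera or control yaw), while others use owner yaw.
; The construction script applies the supplied sprite, and an event toggles visibility.
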(event `/Game/Smartphone/BP/AutomaticMinimap/Blueprints/BP_AutoMap_Interface.SetNewIconVisibility`
  (params (NewValue :type Boolean))
  (`self.SetActorHiddenInGame` (not NewValue)))

(event `self.ReceiveBeginPlay`
  (bind _returnvalue (`KismetStringLibrary.GetCharacterArrayFromString` (`KismetSystemLibrary.GetDisplayName` self)))
  (bind _output (`|GetArrayItem` _returnvalue (`KismetArrayLibrary.Array_LastIndex` _returnvalue)))
  (if (`KismetStringLibrary.IsNumeric` _output)
    (set `self.Index` (`KismetStringLibrary.GetCharacterAsNumber` _output))
    (else
      (set `self.Index` 0)))
  (`KismetSystemLibrary.Delay` 0.1)
  (set `self.RotRule` (`/Game/Smartphone/UMG/AutomaticMinimap/UMG_Minimap.PawnIconsRotationRule` (`/Game/Smartphone/BP/AutomaticMinimap/Blueprints/BP_AutoMinimapSceneCapture.Minimap` (`self.SceneCaptureRef`))))
  (bind _aspawn (cast `Pawn` (`self.OwnerActor`)))
  (set `self.Pawn` _aspawn)
  (set `self.PawnRotation` true))

(event `self.ReceiveTick`
  (params (DeltaSeconds :type "Float (single-precision)"))
  (bind (_returnvalue_x _returnvalue_y) (`KismetMathLibrary.BreakVector` (`self.K2_GetActorLocation`)))
  (bind _index (`self.Index`))
  (bind (_returnvalue_roll _returnvalue_pitch _returnvalue_yaw) (`KismetMathLibrary.BreakRotator` (`self.K2_GetActorRotation` (`self.OwnerActor`))))
  (`self.K2_SetActorLocation` (`KismetMathLibrary.MakeVector` _returnvalue_x _returnvalue_y (+ -99999.0 (`KismetMathLibrary.SelectFloat` 0.0 (/ 1.0 (`KismetMathLibrary.Conv_IntToDouble` _index)) (== _index 0)))))
  (if (`self.PawnRotation`)
    (bind _pawn (`self.Pawn`)
      (:`then`
        (bind (_returnvalue_roll_2 _returnvalue_pitch_2 _returnvalue_yaw_2) (`KismetMathLibrary.BreakRotator` (`self.K2_GetActorRotation` _pawn)))
        (bind (_returnvalue_roll_3 _returnvalue_pitch_3 _returnvalue_yaw_3) (`KismetMathLibrary.BreakRotator` (`Pawn.GetControlRotation` _pawn)))
        (`self.K2_SetActorRotation` (`KismetMathLibrary.MakeRotator` 90.0 0.0 (select `/Game/Smartphone/ENUMs/ENUM_MinimapRotationRule` (`self.RotRule`) :`NewEnumerator1` _returnvalue_yaw_2 :`NewEnumerator2` (.yaw (`.OutRotation` (`self.GetActorEyesViewPoint` _pawn))) :`NewEnumerator3` _returnvalue_yaw_3))))
      (:`else`))
    (else
      (`self.K2_SetActorRotation` (`KismetMathLibrary.MakeRotator` 90.0 0.0 _returnvalue_yaw)))))

(fn `UpdateMinimapSIzeBeforeFullscreen`
  (returns (NewVal :type "Vector2D Structure"))
  (return (0.0 0.0)))

(fn `UserConstructionScript`
  (bind _inicon (`self.InIcon`)
    (:`then`
      (`PaperSpriteComponent.SetSprite` (`self.T_Player_Icon_Sprite`) _inicon))
    (:`else`)))