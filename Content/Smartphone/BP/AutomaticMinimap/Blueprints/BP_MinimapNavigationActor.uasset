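; Minimap navigation actor that draws a navmesh route from its owning pawn to a target actor or fixed point.
; Builds spline meshes along the path, moved far below the world to show only in the minimap's scene capture.
; Each tick it re-queries the path, moving existing meshes or rebuilding when the point count changes.
; It asks the minimap renderer to discard navigation on arrival or when the followed actor becomes invalid.
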(event `self.ReceiveBeginPlay`)

(event `self.ReceiveTick`
  (params (DeltaSeconds :type "Float (single-precision)"))
  (bind (_target_x _target_y) (`KismetMathLibrary.BreakVector` (`self.Target`)))
  (bind (_returnvalue_x _returnvalue_y) (`KismetMathLibrary.BreakVector` (`self.K2_GetActorLocation` (`self.TargetActor`))))
  (bind (_returnvalue_x_2 _returnvalue_y_2) (`KismetMathLibrary.BreakVector` (`self.K2_GetActorLocation` (`self.GetOwner`))))
  (bind (_returnvalue_x_3 _returnvalue_y_3) (`KismetMathLibrary.BreakVector` (`self.K2_GetActorLocation` (`self.GetOwner`))))
  (if (`self.PathWasBuilt`)
    (`|ExecutionSequence`
      (:`then_0`
        (`self.UpdatePath`))
      (:`then_1`
        (if (`self.Should Follow Actor`)
          (if (<= (`KismetMathLibrary.VSize` (- (`KismetMathLibrary.MakeVector` _returnvalue_x_2 _returnvalue_y_2) (`KismetMathLibrary.MakeVector` _returnvalue_x _returnvalue_y))) (`self.AcceptableRadius`))
            (`self.Discard`))
          (elif (<= (`KismetMathLibrary.VSize` (- (`KismetMathLibrary.MakeVector` _returnvalue_x_3 _returnvalue_y_3) (`KismetMathLibrary.MakeVector` _target_x _target_y))) (`self.AcceptableRadius`))
            (`self.Discard`)))))))

(fn `RebuildPath`
  (params (DestroyOldMeshes :type Boolean))
  (locals (`Last Mesh` :type "SplineMeshComponent Object Reference") (i :type Integer))
  (bind (_returnvalue_x _returnvalue_y) (`KismetMathLibrary.BreakVector` (`SceneComponent.K2_GetComponentLocation` (`local.Last Mesh`))))
  (bind (_start _starttan _end _endtan) (`self.GetSplineStartEnd` (`local.i`)))
  (`SplineComponent.SetSplinePoints` (`self.Spline`) (`self.CurrentPath`) "World" true)
  (if DestroyOldMeshes
    (for _array_element (`self.Meshes`)
      (`ActorComponent.K2_DestroyComponent` _array_element))
    (`KismetArrayLibrary.Array_Clear` (`self.Meshes`)))
  (`|ExecutionSequence`
    (:`then_0`
      (for (_ _array_index) (`self.CurrentPath`)
        (bind _output_get (set `local.i` _array_index))
        (if (!= _output_get (`KismetArrayLibrary.Array_LastIndex` (`self.CurrentPath`)))
          (bind _returnvalue (`AddComponent|NODE_AddSplineMeshComponent-0` :`RelativeTransform` (`KismetMathLibrary.MakeTransform` (0.0 0.0 1.0))))
          (bind _output_get_2 (set `local.Last Mesh` _returnvalue))
          (`KismetArrayLibrary.Array_Add` (`self.Meshes`) _output_get_2)
          (`SplineMeshComponent.SetStartAndEnd` (`local.Last Mesh`) _start _starttan _end _endtan true)
          (`self.UpDirFic` (`local.Last Mesh`) (`local.i`))
          (`SceneComponent.K2_SetWorldLocation` (`local.Last Mesh`) (`KismetMathLibrary.MakeVector` _returnvalue_x _returnvalue_y -9999.0) false false) ; The actual spline mesh should not be visible in the game but still be rendered by the SceneCaptureComponent
        )))
    (:`then_1`
      (set `self.PathWasBuilt` true))))

(fn `UpdatePath`
  (locals (LocalLastPath :type "NavigationPath Object Reference"))
  (bind _highqualitypath (`self.HighQualityPath`))
  (bind _highqualitypath_2 (`self.HighQualityPath`))
  (bind _returnvalue (`self.K2_GetActorLocation` (`self.GetOwner`)))
  (bind _projectedlocation (`NavigationSystemV1.K2_ProjectPointToNavigation` (`self.K2_GetActorLocation` (`self.GetOwner`)) null "/Script/NavigationSystem.RecastFilter_UseDefaultArea" (9999.0 9999.0 9999.0)))
  (if (and (`self.Should Follow Actor`) (not (`KismetSystemLibrary.IsValid` (`self.TargetActor`))))
    (`self.Discard`)
    (else
      (if (`self.Should Follow Actor`)
        (bind _returnvalue_2 (`NavigationSystemV1.FindPathToLocationSynchronously` _projectedlocation (`NavigationSystemV1.K2_ProjectPointToNavigation` (`self.K2_GetActorLocation` (`self.TargetActor`)) null "/Script/NavigationSystem.RecastFilter_UseDefaultArea" (9999.0 9999.0 9999.0)) null "/Script/NavigationSystem.RecastFilter_UseDefaultArea"))
        (set `local.LocalLastPath` _returnvalue_2)
        (else
          (bind _returnvalue_3 (`NavigationSystemV1.FindPathToLocationSynchronously` _projectedlocation (`self.Target`) null "/Script/NavigationSystem.RecastFilter_UseDefaultArea"))
          (set `local.LocalLastPath` _returnvalue_3)))
      (bind _lastpath (`self.LastPath`)
        (:`then`
          (if (or (> (`KismetMathLibrary.VSize` (- (`|GetArrayItem` (`NavigationPath.PathPoints` _lastpath)) _returnvalue)) (`KismetMathLibrary.VSize` (- (`|GetArrayItem` (`NavigationPath.PathPoints` (`local.LocalLastPath`))) _returnvalue))) (== (`NavigationPath.GetPathLength` _lastpath) -1.0))
            (bind _output_get (set `self.LastPath` (`local.LocalLastPath`)))
            (if (== (`KismetArrayLibrary.Array_Length` (`NavigationPath.PathPoints` _output_get)) (`KismetArrayLibrary.Array_Length` (`self.CurrentPath`)))
              (bind _output_get_2 (set `self.CurrentPath` (`NavigationPath.PathPoints` (`local.LocalLastPath`))))
              (`SplineComponent.SetSplinePoints` (`self.Spline`) _output_get_2 "World" true)
              (for (_array_element _array_index) (`self.Meshes`)
                (bind (_start _starttan _end _endtan) (`self.GetSplineStartEndAtTime` _array_index))
                (bind (_start_2 _starttan_2 _end_2 _endtan_2) (`self.GetSplineStartEnd` _array_index))
                (`SplineMeshComponent.SetStartAndEnd` _array_element (`KismetMathLibrary.SelectVector` _start _start_2 _highqualitypath_2) (`KismetMathLibrary.SelectVector` _starttan _starttan_2 _highqualitypath_2) (`KismetMathLibrary.SelectVector` _end _end_2 _highqualitypath) (`KismetMathLibrary.SelectVector` _endtan _endtan_2 _highqualitypath) true)
                (`self.UpDirFic` _array_element _array_index (`self.HighQualityPath`)))
              (else
                (set `self.CurrentPath` (`NavigationPath.PathPoints` (`local.LocalLastPath`)))
                (`self.RebuildPath` true)))))
        (:`else`
          (set `self.LastPath` (`local.LocalLastPath`)))))))

(fn `UserConstructionScript`
  (set `self.Should Follow Actor` (`KismetSystemLibrary.IsValid` (`self.TargetActor`)))
  (`self.UpdateTarget`)
  (if (> (`KismetArrayLibrary.Array_Length` (`self.CurrentPath`)) 0)
    (`self.RebuildPath` false)))