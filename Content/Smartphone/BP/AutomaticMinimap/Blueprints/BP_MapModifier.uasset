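; BP_MapModifier is a minimap modifier zone that changes how the map renders while a player pawn overlaps it.
; On entry, it finds the pawn's UMG_Minimap by owning pawn, caches its render actor's TraceHeight, optionally overrides that height, and hides the HideActorsOnOverlap actors from the map.
; On exit, it restores the cached height from the MapActorsInside map and shows those actors again.
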(event `self.ReceiveBeginPlay`)

(event `self.ReceiveActorBeginOverlap`
  (params (OtherActor :type "Actor Object Reference"))
  (bind _array_element (`self.ActorHasMinimapWidget?` OtherActor)
    (:`Found it`
      (bind _output_get (set `self.LastWidget` _array_element))
      (bind _renderactor (`/Game/Smartphone/UMG/AutomaticMinimap/UMG_Minimap.RenderActor` _output_get)
        (:`then`
          (`BlueprintMapLibrary.Map_Add` (`self.MapActorsInside`) _renderactor (`/Game/Smartphone/BP/AutomaticMinimap/Blueprints/BP_AutoMinimapSceneCapture.bTraceHeight` _renderactor))
          (`self.ProccessRenderActor`))
        (:`else`)))))

(event `self.ReceiveActorEndOverlap`
  (params (OtherActor :type "Actor Object Reference"))
  (bind _array_element (`self.ActorHasMinimapWidget?` OtherActor)
    (:`Found it`
      (bind _output_get (set `self.LastWidget` _array_element))
      (bind _keys (`BlueprintMapLibrary.Map_Keys` (`self.MapActorsInside`)))
      (bind _renderactor (`/Game/Smartphone/UMG/AutomaticMinimap/UMG_Minimap.RenderActor` _output_get))
      (bind _returnvalue (`KismetArrayLibrary.Array_Find` _keys _renderactor))
      (if (!= _returnvalue -1)
        (bind _values (`BlueprintMapLibrary.Map_Values` (`self.MapActorsInside`)))
        (set `/Game/Smartphone/BP/AutomaticMinimap/Blueprints/BP_AutoMinimapSceneCapture.bTraceHeight` (`|GetArrayItem` _values _returnvalue) (`|GetArrayItem` _keys _returnvalue))
        (`BlueprintMapLibrary.Map_Remove` (`self.MapActorsInside`) _renderactor)
        (`/Game/Smartphone/UMG/AutomaticMinimap/UMG_Minimap.ShowActorsOnMinimap` (`self.LastWidget`) (`self.HideActorsOnOverlap`))))))

(fn `UserConstructionScript`)